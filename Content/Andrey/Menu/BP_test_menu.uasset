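; Test menu actor that spawns detail actors into the scene at its StaticMesh's world location.
; PressButton stores a count and detail number, then loops that many times, spawning the class picked from the Class array by that number.
; BeginPlay runs the same spawn step once.
; Debug "Hello" prints trace each step, and a spaced-row position calculation is left unconnected, so all spawns share one point.
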(event EventPressButton
  (params (Count :type Integer) (DetailNumber :type Integer) (time :type Integer))
  (Development|PrintString "Hello")
  ;[1 1 1] Появление деталей на сцене
  (Variables|Default|SetNumberDetail DetailNumber)
  (Variables|Default|SetNumberOfPrints Count)
  (for _index (range 0 (- (Variables|Default|GetNumberOfPrints) 1))
    (Development|PrintString "Hello")
    (Game|SpawnActorfromClass (Utilities|Array|Get(acopy) (Variables|Default|GetClass) (Variables|Default|GetNumberDetail)) (Math|Transform|MakeTransform (Transformation|GetWorldLocation (Variables|Default|GetStaticMesh)) "0, 0, 0" "1,1,1") "Undefined" 0 0)
    (Development|PrintString "Hello")))

(event EventBeginPlay
  (Development|PrintString "Hello")
  ;[1 1 1] Появление деталей на сцене
  (Game|SpawnActorfromClass (Utilities|Array|Get(acopy) (Variables|Default|GetClass) (Variables|Default|GetNumberDetail)) (Math|Transform|MakeTransform (Transformation|GetWorldLocation (Variables|Default|GetStaticMesh)) "0, 0, 0" "1,1,1") "Undefined" 0 0)
  (Development|PrintString "Hello"))

(fn ConstructionScript)