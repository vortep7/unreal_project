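; 3D printer actor that prints a chosen number of detail actors and moves them to inventory or trash locations.
; PressButton plays the printer animation, waits, spawns the selected class in a spaced row with timeline scale-up and Niagara effect, then blocks further printing.
; CheckTeleport moves prints to the inventory point, or to trash on pop or overflow, and re-enables printing.
; A growing ZOV offset, never reset here, spaces moved items and triggers overflow.
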(event EventCheckTeleport
  (params (Add_Button :type Boolean) (Pop_Button :type Boolean))
  (bind _teleportlocation (Variables|Default|GetTeleportLocation))
  (bind _pop_location (Variables|Default|GetPop_location))
  (bind _returnvalue (Transformation|GetWorldLocation _pop_location))
  (bind _returnvalue_2 (Transformation|GetWorldLocation _teleportlocation))
  (bind _output_get (Variables|Default|SetAdd_Button Add_Button))
  (bind _output_get_2 (Variables|Default|SetPop_Button Pop_Button))
  (if (Math|Boolean|Equal(Boolean) _output_get true)
    (if (> (Variables|Default|GetZOV) 1e+02)
      (Development|PrintString "Инвентарь переполнен, объект отправлен в мусорку" true true "(R=0.000000,G=0.660000,B=1.000000,A=1.000000)" 1e+01)
      (for _index (range 0 (- (Variables|Default|GetNumberOfPrints) 1)) :!label _label
        (Transformation|Teleport (Utilities|Array|Get(acopy) (Variables|Default|GetSpawned_Actor) _index) (Math|Vector|MakeVector (.x _returnvalue) (+ (* _index (Variables|Default|GetSpacing)) (+ (.y _returnvalue) (Variables|Default|GetZOV)) (Variables|Default|GetZeroOfSet)) (.z _returnvalue)) "0, 0, 0")
        (Variables|Default|SetZOV (+ (Variables|Default|GetZOV) 4e+01))
        (Variables|Default|SetGoNext true))
      (else
        (for _index_2 (range 0 (- (Variables|Default|GetNumberOfPrints) 1))
          (Transformation|Teleport (Utilities|Array|Get(acopy) (Variables|Default|GetSpawned_Actor) _index_2) (Math|Vector|MakeVector (.x _returnvalue_2) (+ (* _index_2 (Variables|Default|GetSpacing)) (+ (.y _returnvalue_2) (Variables|Default|GetZOV)) (Variables|Default|GetZeroOfSet)) (.z _returnvalue_2)) "0, 0, 0")
          (Variables|Default|SetZOV (+ (Variables|Default|GetZOV) 4e+01))
          (Variables|Default|SetGoNext true))))
    (elif (Math|Boolean|Equal(Boolean) _output_get_2 true)
      (goto _label))))

(event EventPressButton
  (params (Count :type Integer) (DetailNumber :type Integer) (time :type Integer))
  (bind _scene (Variables|Default|GetScene))
  (bind _returnvalue (Transformation|GetWorldLocation _scene))
  (if (Math|Boolean|Equal(Boolean) true (Variables|Default|GetGoNext))
    (Variables|Default|SetNumberDetail DetailNumber)
    (Variables|Default|SetNumberOfPrints Count)
    (Components|Animation|PlayAnimation (Variables|Default|GetSkeletalMesh) "/Game/Resources/Meshes/3D-Printer_A_Anim.3D-Printer_A_Anim" false)
    (Utilities|FlowControl|Delay (Math|Conversions|ToFloat(Integer) time))
    (for _index (range 0 (- (Variables|Default|GetNumberOfPrints) 1))
      (bind _returnvalue_2 (Game|SpawnActorfromClass (Utilities|Array|Get(acopy) (Variables|Default|GetClass) (Variables|Default|GetNumberDetail)) (Math|Transform|MakeTransform (Math|Vector|MakeVector (.x _returnvalue) (+ (* _index (Variables|Default|GetSpacing)) (.y _returnvalue) (Variables|Default|GetZeroOfSet)) (.z _returnvalue)) "0, 0, 0" "1,1,1") "Undefined" 0 0))
      (bind _scalealpha (Timeline|Timeline_0 Play)
        (:Update
          (Transformation|SetActorScale3D _returnvalue_2 (Math|Vector|MakeVector _scalealpha _scalealpha _scalealpha))
          (Utilities|Array|SetArrayElem (Variables|Default|GetSpawned_Actor) _index _returnvalue_2 true)
          (Components|Activation|Activate (Variables|Default|GetNS_SpawnObject) false)
          (Audio|Components|Audio|Stop (Variables|Default|GetSkeletalMesh))
          (Variables|Default|SetGoNext false))))
    (else
      (Development|PrintString "Убери предмет с принтера"))))

(fn ConstructionScript)